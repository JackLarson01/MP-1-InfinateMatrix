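; BP_Enemy is a short-lived enemy actor that destroys itself after five seconds or when its collision overlaps a projectile or the player.
; A projectile hit destroys both the enemy and the projectile.
; A player hit either triggers the restart display and death flag on the last health point, or shows a Flash widget, lowers score and health, and updates their HUD text directly.
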(event `self.ReceiveBeginPlay`
  (`self.SetLifeSpan` 5.0))

(event `self.ReceiveTick`
  (params (DeltaSeconds :type "Float (single-precision)")))

(event `self.Collision.OnComponentBeginOverlap`
  (params (OverlappedComponent :type "PrimitiveComponent Object Reference") (OtherActor :type "Actor Object Reference") (OtherComp :type "PrimitiveComponent Object Reference") (OtherBodyIndex :type Integer) (bFromSweep :type Boolean) (SweepResult :type "HitResult Structure (by ref)"))
  (bind _asbp_projectiles (cast `/Game/InfiniteMatrix/Blueprints/BP_Projectiles` OtherActor)
    (:`then`
      (`self.K2_DestroyActor`)
      (`self.K2_DestroyActor` _asbp_projectiles))
    (:`CastFailed`
      (bind _asbp_player (cast `/Game/InfiniteMatrix/Blueprints/BP_Player` OtherActor))
      (bind _returnvalue (- (`/Game/InfiniteMatrix/Blueprints/BP_Player.PlayerHealth` _asbp_player) 1.0))
      (if (== _returnvalue 0.0)
        (`/Game/InfiniteMatrix/Blueprints/BP_Player.DisplayRestart` _asbp_player)
        (set `/Game/InfiniteMatrix/Blueprints/BP_Player.IsDead` true _asbp_player)
        (`self.K2_DestroyActor`)
        (else
          (`self.K2_DestroyActor`)
          (bind _returnvalue_2 (`|CreateWidget` "/Game/InfiniteMatrix/UI/Flash.Flash_C"))
          (`UserWidget.AddToViewport` _returnvalue_2 0)
          (set `/Game/InfiniteMatrix/Blueprints/BP_Player.Score` (- (`/Game/InfiniteMatrix/Blueprints/BP_Player.Score` _asbp_player) 20) _asbp_player)
          (`TextBlock.SetText` (`/Game/InfiniteMatrix/UI/ScoreText.ScoreText` (`/Game/InfiniteMatrix/Blueprints/BP_Player.LocalScoreText` _asbp_player)) (`KismetTextLibrary.Conv_StringToText` (`KismetStringLibrary.Concat_StrStr` "Score: " (`KismetStringLibrary.Conv_IntToString` (`/Game/InfiniteMatrix/Blueprints/BP_Player.Score` _asbp_player)))))
          (bind _output_get (set `/Game/InfiniteMatrix/Blueprints/BP_Player.PlayerHealth` _returnvalue _asbp_player))
          (`TextBlock.SetText` (`/Game/InfiniteMatrix/Blueprints/BP_Player.LocalHealthText` _asbp_player) (`KismetTextLibrary.Conv_StringToText` (`KismetStringLibrary.Concat_StrStr` "Health: " (`KismetStringLibrary.Conv_IntToString` (`KismetMathLibrary.FTrunc` _output_get))))))))))

(fn `UserConstructionScript`)