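; BP_Ammo_Pickup is a short-lived ammo pickup that expires five seconds after it spawns.
; When BP_Player overlaps its Sphere component, it adds a fixed amount to the player's Ammo and destroys itself.
; It also writes the new count directly into the player's AmmoText widget instead of leaving the display update to the player.
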(event `self.ReceiveBeginPlay`
  (`parent.ReceiveBeginPlay`)
  (`self.SetLifeSpan` 5.0))

(event `self.Sphere.OnComponentBeginOverlap`
  (params (OverlappedComponent :type "PrimitiveComponent Object Reference") (OtherActor :type "Actor Object Reference") (OtherComp :type "PrimitiveComponent Object Reference") (OtherBodyIndex :type Integer) (bFromSweep :type Boolean) (SweepResult :type "HitResult Structure (by ref)"))
  (bind _asbp_player (cast `/Game/InfiniteMatrix/Blueprints/BP_Player` OtherActor))
  (bind _output_get (set `/Game/InfiniteMatrix/Blueprints/BP_Player.Ammo` (+ (`/Game/InfiniteMatrix/Blueprints/BP_Player.Ammo` _asbp_player) 10) _asbp_player))
  (`TextBlock.SetText` (`/Game/InfiniteMatrix/UI/Ammo_Text.ScoreText_1` (`/Game/InfiniteMatrix/Blueprints/BP_Player.AmmoText` _asbp_player)) (`KismetTextLibrary.Conv_StringToText` (`KismetStringLibrary.Concat_StrStr` "Ammo: " (`KismetStringLibrary.Conv_IntToString` _output_get))))
  (`self.K2_DestroyActor`))

(fn `UserConstructionScript`
  (`parent.UserConstructionScript`))